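; BP_Spawner is an enemy spawner that creates AI pawns at the location and rotation of its Arrow component.
; Spawn takes an override spawn group and, when valid, spawns each valid entry's class by its count.
; An invalid group falls back to the spawner's own SpawnClass and NumToSpawn.
; Each pawn is added uniquely to SpawnedPawns, which accumulates across calls and is returned.
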(fn `Spawn`
  (params (OverrideSpawnData :type "/Game/FGShooter/Enemies/FSpawnGroup Structure"))
  (returns (ReturnValue :type "Array of Pawn Object Reference"))
  (locals (SpawnedPawns :type "Array of Pawn Object Reference"))
  (bind _arrow (`self.Arrow`))
  (bind _arrow_2 (`self.Arrow`))
  (if (`/Game/FGShooter/Core/BPF_Utilities.IsValidSpawnGroup` OverrideSpawnData)
    (for _array_element (`.SpawnGroup_3_7214EF8640147EA60D39ABBE583C093D` (break `/Game/FGShooter/Enemies/FSpawnGroup` OverrideSpawnData))
      (if (`/Game/FGShooter/Core/BPF_Utilities.IsValidSpawnData` _array_element)
        (bind (_class _numtospawn) (break `/Game/FGShooter/Enemies/FSpawnData` _array_element))
        (for _ (range _numtospawn)
          (bind _returnvalue (`AIBlueprintHelperLibrary.SpawnAIFromClass` _class null (`SceneComponent.K2_GetComponentLocation` _arrow_2) (`SceneComponent.K2_GetComponentRotation` _arrow_2)))
          (`KismetArrayLibrary.Array_AddUnique` (`local.SpawnedPawns`) _returnvalue))))
    (return (`local.SpawnedPawns`))
    (else
      (for _ (range (`self.NumToSpawn`))
        (bind _returnvalue_2 (`AIBlueprintHelperLibrary.SpawnAIFromClass` (`self.SpawnClass`) null (`SceneComponent.K2_GetComponentLocation` _arrow) (`SceneComponent.K2_GetComponentRotation` _arrow)))
        (`KismetArrayLibrary.Array_AddUnique` (`local.SpawnedPawns`) _returnvalue_2))
      (return (`local.SpawnedPawns`)))))

(fn `UserConstructionScript`)