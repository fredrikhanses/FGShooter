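; AI controller for sniper enemies that runs the BT_EnemySniper behavior tree on possession.
; It binds to the possessed BP_EnemyBase's OnKilled event to set the IsDead blackboard key.
; AI Perception updates set HasLineOfSight and TargetPlayer when the player is sensed.
; Any other perception update starts a grace timer that clears both keys on expiry, and sensing the player again cancels it.
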(event `self.ReceivePossess`
  (params (PossessedPawn :type "Pawn Object Reference"))
  (`self.RunBehaviorTree` "/Game/FGShooter/Enemies/BT_EnemySniper.BT_EnemySniper")
  (`BlackboardComponent.SetValueAsBool` (`self.Blackboard`) "IsDead" false)
  (bind _asbp_enemy_base (cast `/Game/FGShooter/Enemies/BP_EnemyBase` PossessedPawn))
  (add `/Game/FGShooter/Enemies/BP_EnemyBase.OnKilled` _asbp_enemy_base (delegate `OnKilled_Event_0`)))

(event `OnKilled_Event_0`
  (params (KilledEnemy :type "/Game/FGShooter/Enemies/BP_EnemyBase Object Reference"))
  (`BlackboardComponent.SetValueAsBool` (`self.Blackboard`) "IsDead" true))

(event `self.AIPerception.OnTargetPerceptionUpdated`
  (params (Actor :type "Actor Object Reference") (Stimulus :type "AIStimulus Structure"))
  (bind _blackboard (`self.Blackboard`))
  (if (and (== Actor (`GameplayStatics.GetPlayerCharacter` 0)) (`.bSuccessfullySensed` (break `AIStimulus` Stimulus)))
    (`KismetSystemLibrary.K2_ClearAndInvalidateTimerHandle` (`self.EnemyTimer`))
    (`BlackboardComponent.SetValueAsBool` _blackboard (`self.HasLineOfSight`) true)
    (`BlackboardComponent.SetValueAsObject` _blackboard (`self.TargetPlayer`) Actor)
    (else
      (bind _returnvalue (`KismetSystemLibrary.K2_SetTimerDelegate` (delegate `StartEnemyTimer`) (`self.LineOfSightTimer`)))
      (set `self.EnemyTimer` _returnvalue))))

(event `StartEnemyTimer`
  (bind _blackboard (`self.Blackboard`))
  (`BlackboardComponent.SetValueAsBool` _blackboard (`self.HasLineOfSight`) false)
  (`BlackboardComponent.SetValueAsObject` _blackboard (`self.TargetPlayer`) null))

(fn `UserConstructionScript`)