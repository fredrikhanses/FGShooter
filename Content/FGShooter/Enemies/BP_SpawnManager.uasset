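; BP_SpawnManager distributes an enemy group across a set of spawners.
; Spawn uses the override spawn data when it is valid, otherwise the group from EnemyGroup.
; Entries go to Spawners round-robin by index modulo, each wrapped as a single-entry spawn group in a SpawnMessage call.
; The results accumulate in SpawnedPawns, which Spawn returns.
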(fn `Spawn`
  (params (OverrideSpawnData :type "/Game/FGShooter/Enemies/FSpawnGroup Structure"))
  (returns (ReturnValue :type "Array of Pawn Object Reference"))
  (locals (SpawnedPawns :type "Array of Pawn Object Reference"))
  (for (_array_element _array_index) (`.SpawnGroup_3_7214EF8640147EA60D39ABBE583C093D` (break `/Game/FGShooter/Enemies/FSpawnGroup` (select `bool` (`/Game/FGShooter/Core/BPF_Utilities.IsValidSpawnGroup` OverrideSpawnData) :`false` (`/Game/FGShooter/Enemies/SpawnGroupDataTemplate.SpawnGroup` (`self.EnemyGroup`)) :`true` OverrideSpawnData)))
    (bind _returnvalue (message `/Game/FGShooter/Core/BPI_Spawnable.Spawn` (`|GetArrayItem` (`self.Spawners`) (mod _array_index (`KismetArrayLibrary.Array_Length` (`self.Spawners`)))) (make `/Game/FGShooter/Enemies/FSpawnGroup` (`|MakeArray` _array_element))))
    (`KismetArrayLibrary.Array_Append` (`local.SpawnedPawns`) _returnvalue))
  (return (`local.SpawnedPawns`)))

(fn `UserConstructionScript`)