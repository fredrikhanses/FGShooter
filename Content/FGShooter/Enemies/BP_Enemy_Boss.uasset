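; BP_Enemy_Boss is the boss enemy in FGShooter, damaging the player on contact and awarding score.
; A capsule hit applies TouchDamage only when the other actor's class is exactly FirstPersonCharacter, crediting the boss's controller as instigator.
; Its AddScore event passes ScoreToAdd to BP_GameState; nothing in this graph calls that event.
; The construction script only runs the parent's version.
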(event `self.CapsuleComponent.OnComponentHit`
  (params (HitComponent :type "PrimitiveComponent Object Reference") (OtherActor :type "Actor Object Reference") (OtherComp :type "PrimitiveComponent Object Reference") (NormalImpulse :type "Vector Structure") (Hit :type "HitResult Structure (by ref)"))
  ;[1 1 1] Damage player on touch
  (if (== (`GameplayStatics.GetObjectClass` OtherActor) "/Game/FGShooter/Player/FirstPersonCharacter.FirstPersonCharacter_C")
    (`GameplayStatics.ApplyDamage` OtherActor (`self.TouchDamage`) (`self.GetController`) self)))

(event `self.Add Score`
  (params (ScoreToAdd :type Integer))
  ;[1 1 1] Add score for Boss
  (bind _asbp_game_state (cast `/Game/FGShooter/Core/BP_GameState` (`GameplayStatics.GetGameState`)))
  (`/Game/FGShooter/Core/BP_GameState.AddScore` _asbp_game_state (`self.ScoreToAdd`)))

(fn `UserConstructionScript`
  (`parent.UserConstructionScript`))