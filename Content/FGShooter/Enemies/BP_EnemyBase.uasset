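; Base enemy character that punches for damage, takes projectile hits and drops a pickup when destroyed.
; Mesh and hand hits apply the player projectile's damage, each toggling its own FlipFlop between ammo and health pickup.
; Punch briefly enables hand collision, and hand overlaps deal damage gated by a shared cooldown.
; At zero health it explodes, hides, adds score through BP_GameState and sets a short lifespan, whose expiry spawns the pickup.
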(event `self.LeftHand.OnComponentHit`
  (params (HitComponent :type "PrimitiveComponent Object Reference") (OtherActor :type "Actor Object Reference") (OtherComp :type "PrimitiveComponent Object Reference") (NormalImpulse :type "Vector Structure") (Hit :type "HitResult Structure (by ref)"))
  ;[1 1 1] Player shoots enemy. Set type of pickup
  (bind _damagedealt (`self.IsPlayerProjectile` OtherActor))
  (`/Engine/EditorBlueprintResources/StandardMacros.FlipFlop`
    (:`A`
      (set `self.PickupType` "/Game/FGShooter/Objects/BP_AmmoPickup.BP_AmmoPickup_C"))
    (:`B`
      (set `self.PickupType` "/Game/FGShooter/Objects/BP_HealthPickup.BP_HealthPickup_C")))
  (`GameplayStatics.ApplyDamage` self _damagedealt))

(event `DamageTimer`
  ;[1 1 1] Damage Player timer
  (`KismetSystemLibrary.Delay` (`self.DamagePlayerInterval`))
  (set `self.bCanDamagePlayer` true))

(event `self.RightHand.OnComponentHit`
  (params (HitComponent :type "PrimitiveComponent Object Reference") (OtherActor :type "Actor Object Reference") (OtherComp :type "PrimitiveComponent Object Reference") (NormalImpulse :type "Vector Structure") (Hit :type "HitResult Structure (by ref)"))
  ;[1 1 1] Player shoots enemy. Set type of pickup
  (bind _damagedealt (`self.IsPlayerProjectile` OtherActor))
  (`/Engine/EditorBlueprintResources/StandardMacros.FlipFlop`
    (:`A`
      (set `self.PickupType` "/Game/FGShooter/Objects/BP_AmmoPickup.BP_AmmoPickup_C"))
    (:`B`
      (set `self.PickupType` "/Game/FGShooter/Objects/BP_HealthPickup.BP_HealthPickup_C")))
  (`GameplayStatics.ApplyDamage` self _damagedealt))

(event `self.ReceiveBeginPlay`
  ;[1 1 1] Apply damage and check if dead
  (add `self.OnTakeAnyDamage` (delegate `OnTakeAnyDamage_Event_0`))
  (add `self.OnDestroyed` (delegate `OnDestroyed_Event_0`)))

(event `Punch`
  (params (Duration :type "Float (double-precision)"))
  ;[1 1 1] Punch
  (set `self.bIsPunching` true)
  (`PrimitiveComponent.SetCollisionEnabled` (`self.LeftHand`) "QueryAndPhysics")
  (`PrimitiveComponent.SetCollisionEnabled` (`self.RightHand`) "QueryAndPhysics")
  (`KismetSystemLibrary.Delay` 2.0)
  (set `self.bIsPunching` false)
  (`PrimitiveComponent.SetCollisionEnabled` (`self.LeftHand`) "NoCollision")
  (`PrimitiveComponent.SetCollisionEnabled` (`self.RightHand`) "NoCollision"))

(event `OnTakeAnyDamage_Event_0` :!signature `self.OnTakeAnyDamage`
  (params (DamagedActor :type "Actor Object Reference") (Damage :type "Float (double-precision)") (DamageType :type "DamageType Object Reference") (InstigatedBy :type "Controller Object Reference") (DamageCauser :type "Actor Object Reference"))
  ;[1 1 1] Apply damage and check if dead
  (set `self.Health` (- (`self.Health`) Damage))
  (if (<= (`self.Health`) 0.0)
    (`self.Die`)))

(event `OnDestroyed_Event_0` :!signature `self.OnDestroyed`
  (params (DestroyedActor :type "Actor Object Reference"))
  ;[1 1 1] Apply damage and check if dead
  (`self.Spawn Goodies`))

(event `self.Mesh.OnComponentHit`
  (params (HitComponent :type "PrimitiveComponent Object Reference") (OtherActor :type "Actor Object Reference") (OtherComp :type "PrimitiveComponent Object Reference") (NormalImpulse :type "Vector Structure") (Hit :type "HitResult Structure (by ref)"))
  ;[1 1 1] Player shoots enemy. Set type of pickup
  (bind _damagedealt (`self.IsPlayerProjectile` OtherActor))
  (`/Engine/EditorBlueprintResources/StandardMacros.FlipFlop`
    (:`A`
      (set `self.PickupType` "/Game/FGShooter/Objects/BP_AmmoPickup.BP_AmmoPickup_C"))
    (:`B`
      (set `self.PickupType` "/Game/FGShooter/Objects/BP_HealthPickup.BP_HealthPickup_C")))
  (`GameplayStatics.ApplyDamage` self _damagedealt))

(event `Add Score`
  (params (ScoreToAdd :type Integer))
  ;[1 1 1] Add default score
  (bind _asbp_game_state (cast `/Game/FGShooter/Core/BP_GameState` (`GameplayStatics.GetGameState`)))
  (`/Game/FGShooter/Core/BP_GameState.AddScore` _asbp_game_state ScoreToAdd))

(event `self.LeftHand.OnComponentBeginOverlap`
  (params (OverlappedComponent :type "PrimitiveComponent Object Reference") (OtherActor :type "Actor Object Reference") (OtherComp :type "PrimitiveComponent Object Reference") (OtherBodyIndex :type Integer) (bFromSweep :type Boolean) (SweepResult :type "HitResult Structure (by ref)"))
  ;[1 1 1] Hit and damage player
  (if (`self.bCanDamagePlayer`)
    (`self.DamageTimer`)
    (`GameplayStatics.ApplyDamage` OtherActor (`self.Damage`) (`self.GetController`) self)
    (set `self.bCanDamagePlayer` false :!label _label)))

(event `Die`
  ;[1 1 1] Enemy explodes and player get score
  (bind _returnvalue (`|SpawnActorFromClass` "/Game/StarterContent/Blueprints/Blueprint_Effect_Explosion.Blueprint_Effect_Explosion_C" (`self.GetTransform` self) "AdjustIfPossibleButAlwaysSpawn" "OverrideRootScale" null null))
  (`self.K2_AttachToActor` _returnvalue self "None" "SnapToTarget" "SnapToTarget" "SnapToTarget" true)
  (`self.SetActorHiddenInGame` true)
  (`self.SetActorEnableCollision` false)
  (`self.Add Score` (`self.DefaultScoreToAdd`))
  (`self.SetLifeSpan` 2.0))

(event `self.RightHand.OnComponentBeginOverlap`
  (params (OverlappedComponent :type "PrimitiveComponent Object Reference") (OtherActor :type "Actor Object Reference") (OtherComp :type "PrimitiveComponent Object Reference") (OtherBodyIndex :type Integer) (bFromSweep :type Boolean) (SweepResult :type "HitResult Structure (by ref)"))
  ;[1 1 1] Hit and damage player
  (if (`self.bCanDamagePlayer`)
    (`self.DamageTimer`)
    (`GameplayStatics.ApplyDamage` OtherActor (`self.Damage`) (`self.GetController`) self)
    (goto _label)))

(event `Spawn Goodies`
  ;[1 1 1] Spawn health or ammo pickup
  (`|SpawnActorFromClass` (`self.PickupType`) (`self.GetTransform` self) "AdjustIfPossibleButAlwaysSpawn" "OverrideRootScale" null null))

(fn `UpdateWalkSpeed`
  (params (NewWalkSpeed :type "Float (double-precision)"))
  (set `CharacterMovementComponent.MaxWalkSpeed` NewWalkSpeed (`self.CharacterMovement`)))

(fn `UserConstructionScript`)