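; Game state for a first-person shooter that tracks score, health and ammo and decides when the game is won or lost.
; Add and remove functions update the values, checking score and health against BP_GameMode thresholds to trigger WinGame, or kill the player and trigger LoseGame.
; Both events check CurrentState against the opposite outcome, show WBP_EndState, then quit after a short delay.
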(event `WinGame`
  ;[1 1 1] Win or Lose game
  (if (not (`|EnumEquality` (`self.CurrentState`) "NewEnumerator0"))
    (bind _returnvalue (`|CreateWidget` "/Game/FGShooter/Core/WBP_EndState.WBP_EndState_C"))
    (bind _output_get (set `/Game/FGShooter/Core/WBP_EndState.EndState` "NewEnumerator1" _returnvalue))
    (set `self.CurrentState` _output_get)
    (`UserWidget.AddToViewport` _returnvalue 0)
    (`KismetSystemLibrary.Delay` 4.0 :!label _label)
    (`KismetSystemLibrary.QuitGame` null "Quit")))

(event `LoseGame`
  ;[1 1 1] Win or Lose game
  (if (not (`|EnumEquality` (`self.CurrentState`) "NewEnumerator1"))
    (bind _returnvalue (`|CreateWidget` "/Game/FGShooter/Core/WBP_EndState.WBP_EndState_C"))
    (bind _output_get (set `/Game/FGShooter/Core/WBP_EndState.EndState` "NewEnumerator0" _returnvalue))
    (set `self.CurrentState` _output_get)
    (`UserWidget.AddToViewport` _returnvalue 0)
    (goto _label)))

(fn `AddAmmo`
  (params (AmmoToAdd :type Integer))
  (returns (Ammo :type Integer))
  (bind _output_get (set `self.Ammo` (+ AmmoToAdd (`self.Ammo`))))
  (if (> _output_get (`self.MaxAmmo`))
    (bind _output_get_2 (set `self.Ammo` (`self.MaxAmmo`)))
    (return _output_get_2)
    (else
      (return (`self.Ammo`)))))

(fn `AddHealth`
  (params (HealthToAdd :type "Float (double-precision)"))
  (returns (Health :type "Float (double-precision)"))
  (set `self.Health` (+ HealthToAdd (`self.Health`)))
  (if (> (`self.Health`) (`self.MaxHealth`))
    (bind _output_get (set `self.Health` (`self.MaxHealth`)))
    (return _output_get)
    (else
      (return (`self.Health`)))))

(fn `AddScore`
  (params (PointsToAdd :type Integer :default 1))
  (returns (Score :type Integer))
  (set `self.Score` (+ PointsToAdd (`self.Score`)))
  (bind _asbp_game_mode (cast `/Game/FGShooter/Core/BP_GameMode` (`GameplayStatics.GetGameMode`))
    (:`then`
      (if (>= (`self.Score`) (`/Game/FGShooter/Core/BP_GameMode.ScoreToWin` _asbp_game_mode))
        (`self.WinGame`)
        (return (`self.Score`))
        (else
          (return (`self.Score`)))))
    (:`CastFailed`
      (return (`self.Score`)))))

(fn `RemoveAmmo`
  (params (AmmoToRemove :type Integer))
  (returns (Ammo :type Integer))
  (bind _output_get (set `self.Ammo` (- (`self.Ammo`) AmmoToRemove)))
  (if (< _output_get 0)
    (set `self.Ammo` 0)
    (return (`self.Ammo`))))

(fn `RemoveHealth`
  (params (HealthToRemove :type "Float (double-precision)"))
  (returns (Health :type "Float (double-precision)"))
  (bind _output_get (set `self.Health` (- (`self.Health`) HealthToRemove)))
  (bind _asbp_game_mode (cast `/Game/FGShooter/Core/BP_GameMode` (`GameplayStatics.GetGameMode`))
    (:`then`
      (if (<= _output_get (`/Game/FGShooter/Core/BP_GameMode.HealthToLose` _asbp_game_mode))
        (set `self.Health` 0.0)
        (if (`self.Alive`)
          (bind _asfirst_person_character (cast `/Game/FGShooter/Player/FirstPersonCharacter` (`GameplayStatics.GetPlayerCharacter` 0))
            (:`then`
              (`/Game/FGShooter/Player/FirstPersonCharacter.Die` _asfirst_person_character)
              (`self.LoseGame`)
              (set `self.Alive` false)
              (return (`self.Health`)))
            (:`CastFailed`
              (return (`self.Health`))))
          (else
            (return (`self.Health`))))
        (else
          (return (`self.Health`)))))
    (:`CastFailed`
      (return (`self.Health`)))))

(fn `UserConstructionScript`)