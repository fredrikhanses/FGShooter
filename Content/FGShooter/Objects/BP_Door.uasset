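; Interactable door that responds only once its linked KeyStone has a key placed, otherwise playing a sound at the player.
; With the key, interaction sends either non-default state back to the first state; no opening by player position is wired.
; TransitionToState lerps the mesh between per-state rotations on a timeline, queuing requests made mid-transition.
; The construction script applies the initial state's rotation.
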(event `/Game/FGShooter/Core/BPI_Interactable.StartInteract`
  ;[1 1 1] Open door based on player relative position or close door when key placed
  (if (`/Game/FGShooter/Objects/BP_KeyStone.KeyPlaced` (`self.KeyStone`))
    (`GameplayStatics.PlaySoundAtLocation` "/Engine/VREditor/Sounds/VR_grab.VR_grab" (`self.K2_GetActorLocation` self) (struct) 1.0 1.0 0.0 null null null)
    (if (or (`|EnumEquality` (`self.State`) "NewEnumerator1") (`|EnumEquality` (`self.State`) "NewEnumerator2"))
      (`self.TransitionToState` "NewEnumerator0")
      (else
        (`self.TransitionToState` (stale `/Game/FGShooter/Core/BPI_Interactable.ChangedDirection` State))))
    (else
      (`GameplayStatics.PlaySoundAtLocation` "/Engine/VREditor/Sounds/UI/Object_Snaps_To_Grid.Object_Snaps_To_Grid" (`self.K2_GetActorLocation` (`GameplayStatics.GetPlayerCharacter` 0)) (struct) 1.0 1.0 0.0 null null null))))

(event `/Game/FGShooter/Core/BPI_Interactable.ChangedDirection`
  (params (State :type "/Game/FGShooter/Core/EDoorState Enum" :default "NewEnumerator0"))
  ;[1 1 1] Open door based on player relative position or close door when key placed
)

(event `TransitionToState`
  (params (TargetState :type "/Game/FGShooter/Core/EDoorState Enum" :default "NewEnumerator0"))
  ;[1 1 1] Animating the door to a target state
  (if (and (`|EnumInequality` TargetState (`self.State`)) (not (`self.bTransitioning`)))
    (set `self.bStateQueued` false)
    (set `self.bTransitioning` true)
    (set `self.TargetState` TargetState)
    (bind (_direction _alpha) (`Timeline|Timeline_0` :!via `PlayFromStart`)
      (:`Update`
        (`SceneComponent.K2_SetRelativeRotation` (`self.SM_Door`) (`KismetMathLibrary.RLerp` (`BlueprintMapLibrary.Map_Find` (`self.TargetRotationByState`) (`self.State`)) (`BlueprintMapLibrary.Map_Find` (`self.TargetRotationByState`) (`self.TargetState`)) _alpha) false false))
      (:`Finished`
        (set `self.State` (`self.TargetState`))
        (set `self.bTransitioning` false)
        (if (`self.bStateQueued`)
          (`self.TransitionToState` (`self.QueuedTargetState`)))))
    (else
      (set `self.QueuedTargetState` TargetState)
      (set `self.bStateQueued` true))))

(fn `UserConstructionScript`
  (`SceneComponent.K2_SetRelativeRotation` (`self.SM_Door`) (`BlueprintMapLibrary.Map_Find` (`self.TargetRotationByState`) (`self.State`)) false false))