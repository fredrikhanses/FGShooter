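; BP_LandMine is a land mine that explodes when hit by either first-person projectile or when the player character overlaps it.
; Explode hides the mine, disables its collision and attaches an explosion effect to it.
; A player trigger also attaches a fire effect to the player and removes health through BP_GameState.
; DestroyMine waits briefly, then destroys the spawned effects and the mine itself.
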(event `Explode`
  ;[1 1 1] Explode mine
  (`self.SetActorHiddenInGame` true)
  (`self.SetActorEnableCollision` false)
  (bind _returnvalue (`|SpawnActorFromClass` "/Game/StarterContent/Blueprints/Blueprint_Effect_Explosion.Blueprint_Effect_Explosion_C" (`self.GetTransform`) "AdjustIfPossibleButAlwaysSpawn" "OverrideRootScale" null null))
  (bind _output_get (set `self.CurrentExplosionEffect` _returnvalue))
  (`self.K2_AttachToActor` _output_get self "None" "SnapToTarget" "SnapToTarget" "SnapToTarget" true))

(event `self.Cube.OnComponentHit`
  (params (HitComponent :type "PrimitiveComponent Object Reference") (OtherActor :type "Actor Object Reference") (OtherComp :type "PrimitiveComponent Object Reference") (NormalImpulse :type "Vector Structure") (Hit :type "HitResult Structure (by ref)"))
  ;[1 1 1] Player shoots mine
  (bind _output_get (set `self.HitActor` OtherActor))
  (bind _returnvalue (`GameplayStatics.GetObjectClass` _output_get))
  (if (or (== _returnvalue "/Game/FGShooter/Player/FirstPersonSecondaryProjectile.FirstPersonSecondaryProjectile_C") (== _returnvalue "/Game/FGShooter/Player/FirstPersonProjectile.FirstPersonProjectile_C"))
    (`self.Explode`)
    (`self.Destroy Mine`)))

(event `Destroy Mine`
  ;[1 1 1] Destroy components
  (`KismetSystemLibrary.Delay` 2.0)
  (`self.K2_DestroyActor` (`self.CurrentExplosionEffect`))
  (set `self.CurrentExplosionEffect` null)
  (if (`KismetSystemLibrary.IsValid` (`self.CurrentFireEffect`))
    (`self.K2_DestroyActor` (`self.CurrentFireEffect`))
    (set `self.CurrentFireEffect` null))
  (set `self.HitActor` null)
  (set `self.OverlapActor` null)
  (`self.K2_DestroyActor`))

(event `self.ReceiveActorBeginOverlap`
  (params (OtherActor :type "Actor Object Reference"))
  ;[1 1 1] Player triggers mine
  (bind _output_get (set `self.OverlapActor` OtherActor))
  (if (== _output_get (`GameplayStatics.GetPlayerCharacter` 0))
    (`self.Explode`)
    (`self.Damage Player`)
    (`self.Destroy Mine`)))

(event `Damage Player`
  ;[1 1 1] Player burns and takes damage
  (bind _returnvalue (`|SpawnActorFromClass` "/Game/StarterContent/Blueprints/Blueprint_Effect_Fire.Blueprint_Effect_Fire_C" (`self.GetTransform` (`self.OverlapActor`)) "AdjustIfPossibleButAlwaysSpawn" "OverrideRootScale" null null))
  (bind _output_get (set `self.CurrentFireEffect` _returnvalue))
  (`self.K2_AttachToActor` _output_get (`self.OverlapActor`) "None" "SnapToTarget" "SnapToTarget" "SnapToTarget" true)
  (bind _asbp_game_state (cast `/Game/FGShooter/Core/BP_GameState` (`GameplayStatics.GetGameState`)))
  (`/Game/FGShooter/Core/BP_GameState.RemoveHealth` _asbp_game_state (`self.Health`)))

(fn `UserConstructionScript`)