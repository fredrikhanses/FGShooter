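; Ammo pickup actor that refills the player's ammo when the player character overlaps it.
; It casts the game state to BP_GameState, which holds the ammo count and cap, and adds its AmmoValue only while ammo is below the max.
; On success it plays a click sound at the player's location and destroys itself; otherwise it stays in the level.
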(event `self.ReceiveActorBeginOverlap`
  (params (OtherActor :type "Actor Object Reference"))
  (if (== OtherActor (`GameplayStatics.GetPlayerCharacter` 0))
    (bind _asbp_game_state (cast `/Game/FGShooter/Core/BP_GameState` (`GameplayStatics.GetGameState`)))
    (if (< (`/Game/FGShooter/Core/BP_GameState.Ammo` _asbp_game_state) (`/Game/FGShooter/Core/BP_GameState.MaxAmmo` _asbp_game_state))
      (`/Game/FGShooter/Core/BP_GameState.AddAmmo` _asbp_game_state (`self.AmmoValue`))
      (`GameplayStatics.PlaySoundAtLocation` "/Engine/VREditor/Sounds/UI/Click_on_Button.Click_on_Button" (`self.K2_GetActorLocation` (`GameplayStatics.GetPlayerCharacter` 0)) (struct) 5.0 1.0 0.0 null null null)
      (`self.K2_DestroyActor`))))

(fn `UserConstructionScript`)