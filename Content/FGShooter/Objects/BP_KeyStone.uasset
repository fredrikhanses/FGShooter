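; BP_KeyStone is an interactable pillar where the player places a key after picking it up.
; On StartInteract, it checks the KeyPickedUp flag on its referenced LootableKey and uses a KeyPlaced flag so placement happens only once.
; Placement unhides its own Key component, enables query-only collision on it and plays a snap sound at the player character's location.
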(event `/Game/FGShooter/Core/BPI_Interactable.StartInteract`
  (bind _key (`self.Key`))
  ;[1 1 1] Put Key on pillar if key picked up
  (if (`/Game/FGShooter/Objects/BP_LootableKey.KeyPickedUp` (`self.LootableKey`))
    (if (not (`self.KeyPlaced`))
      (set `self.KeyPlaced` true)
      (`SceneComponent.SetHiddenInGame` _key false false)
      (`PrimitiveComponent.SetCollisionEnabled` _key "QueryOnly")
      (`GameplayStatics.PlaySoundAtLocation` "/Engine/VREditor/Sounds/UI/Object_Snaps_To_Another_Actor.Object_Snaps_To_Another_Actor" (`self.K2_GetActorLocation` (`GameplayStatics.GetPlayerCharacter` 0)) (struct) 1.0 1.0 0.0 null null null))))

(fn `UserConstructionScript`)