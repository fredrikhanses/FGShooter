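; BP_Laser is a laser hazard that damages the player through BP_GameState on both entering and leaving the beam.
; Shooting the projector reveals its shield while active; once deactivated, a hit makes it explode, award score and destroy itself after a delay.
; Deactivate and Activate events toggle the beam's collision and visibility, with Deactivate also hiding the shield.
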(event `Explode`
  ;[1 1 1] Explode and add score when hit
  (bind _returnvalue (`|SpawnActorFromClass` "/Game/StarterContent/Blueprints/Blueprint_Effect_Explosion.Blueprint_Effect_Explosion_C" (`SceneComponent.K2_GetComponentToWorld` (`self.ExplodePoint`)) "AdjustIfPossibleButAlwaysSpawn" "OverrideRootScale" null null))
  (`self.K2_AttachToActor` _returnvalue self "None" "KeepWorld" "SnapToTarget" "SnapToTarget" true)
  (`self.SetActorHiddenInGame` true)
  (`self.SetActorEnableCollision` false)
  (bind _asbp_game_state (cast `/Game/FGShooter/Core/BP_GameState` (`GameplayStatics.GetGameState`)))
  (`/Game/FGShooter/Core/BP_GameState.AddScore` _asbp_game_state 1)
  (`KismetSystemLibrary.Delay` 4.0)
  (`self.K2_DestroyActor`))

(event `self.Projector.OnComponentHit`
  (params (HitComponent :type "PrimitiveComponent Object Reference") (OtherActor :type "Actor Object Reference") (OtherComp :type "PrimitiveComponent Object Reference") (NormalImpulse :type "Vector Structure") (Hit :type "HitResult Structure (by ref)"))
  (bind _returnvalue (`GameplayStatics.GetObjectClass` OtherActor))
  (bind _shield (`self.Shield`))
  ;[1 1 1] Show shield when hit
  (if (or (== _returnvalue "/Game/FGShooter/Player/FirstPersonProjectile.FirstPersonProjectile_C") (== _returnvalue "/Game/FGShooter/Player/FirstPersonSecondaryProjectile.FirstPersonSecondaryProjectile_C"))
    (if (`self.Deactivated`)
      (`self.Explode`)
      (else
        (`PrimitiveComponent.SetCollisionEnabled` _shield "QueryOnly")
        (`SceneComponent.SetHiddenInGame` _shield false false)))))

(event `self.LaserBeam.OnComponentBeginOverlap`
  (params (OverlappedComponent :type "PrimitiveComponent Object Reference") (OtherActor :type "Actor Object Reference") (OtherComp :type "PrimitiveComponent Object Reference") (OtherBodyIndex :type Integer) (bFromSweep :type Boolean) (SweepResult :type "HitResult Structure (by ref)"))
  ;[1 1 1] Player takes damage when touching laser
  (if (or (== (`GameplayStatics.GetObjectClass` OtherActor) "/Game/FGShooter/Player/FirstPersonCharacter.FirstPersonCharacter_C") (== (`GameplayStatics.GetObjectClass` (stale `self.LaserBeam.OnComponentEndOverlap` OtherActor)) "/Game/FGShooter/Player/FirstPersonCharacter.FirstPersonCharacter_C")) :!label _label
    (bind _asbp_game_state (cast `/Game/FGShooter/Core/BP_GameState` (`GameplayStatics.GetGameState`)))
    (`/Game/FGShooter/Core/BP_GameState.RemoveHealth` _asbp_game_state (`self.Damage`))))

(event `self.LaserBeam.OnComponentEndOverlap`
  (params (OverlappedComponent :type "PrimitiveComponent Object Reference") (OtherActor :type "Actor Object Reference") (OtherComp :type "PrimitiveComponent Object Reference") (OtherBodyIndex :type Integer))
  ;[1 1 1] Player takes damage when touching laser
  (goto _label))

(event `/Game/FGShooter/Core/BPI_Interactable.Deactivate`
  (bind _shield (`self.Shield`))
  (bind _laserbeam (`self.LaserBeam`))
  ;[1 1 1] Deactivate lasers
  (set `self.Deactivated` true)
  (`PrimitiveComponent.SetCollisionEnabled` _shield "NoCollision")
  (`SceneComponent.SetHiddenInGame` _shield true false)
  (`PrimitiveComponent.SetCollisionEnabled` _laserbeam "NoCollision")
  (`SceneComponent.SetHiddenInGame` _laserbeam true false))

(event `/Game/FGShooter/Core/BPI_Interactable.Activate`
  (bind _laserbeam (`self.LaserBeam`))
  ;[1 1 1] Activate lasers
  (set `self.Deactivated` false)
  (`PrimitiveComponent.SetCollisionEnabled` _laserbeam "QueryOnly")
  (`PrimitiveComponent.SetCollisionResponseToAllChannels` _laserbeam "ECR_Overlap")
  (`SceneComponent.SetHiddenInGame` _laserbeam false false))

(fn `UserConstructionScript`)