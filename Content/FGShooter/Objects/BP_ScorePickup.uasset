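; BP_ScorePickup is a pickup actor that awards score to the player.
; When the first player character overlaps it, it adds its Points value to BP_GameState through AddScore.
; It then plays a click sound at the player's location and destroys itself.
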(event `self.ReceiveActorBeginOverlap`
  (params (OtherActor :type "Actor Object Reference"))
  (if (== OtherActor (`GameplayStatics.GetPlayerCharacter` 0))
    (bind _asbp_game_state (cast `/Game/FGShooter/Core/BP_GameState` (`GameplayStatics.GetGameState`)))
    (`/Game/FGShooter/Core/BP_GameState.AddScore` _asbp_game_state (`self.Points`))
    (`GameplayStatics.PlaySoundAtLocation` "/Engine/VREditor/Sounds/VR_click3.VR_click3" (`self.K2_GetActorLocation` (`GameplayStatics.GetPlayerCharacter` 0)) (struct) 1.0 1.0 0.0 null null null)
    (`self.K2_DestroyActor`)))

(fn `UserConstructionScript`)