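; BP_MovingPlatformLong is a moving platform that shuttles back and forth between its starting location and TargetLocation.
; A timeline started on BeginPlay lerps from the current location, rather than the fixed origin, toward the target without sweeping.
; Tick checks for arrival within one unit, then swaps origin and target and replays the timeline.
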(event `self.ReceiveBeginPlay`
  ;[1 1 1] Initial setup and start
  (set `self.OriginalLocation` (`self.K2_GetActorLocation` self))
  (`self.Start Timer`))

(event `Start Timer`
  ;[1 1 1] Start Timer and Move Platform
  (bind (_direction _alpha) (`Timeline|Timeline_0` :!via `PlayFromStart`)
    (:`Update`
      (`self.K2_SetActorLocation` (`KismetMathLibrary.VLerp` (`self.K2_GetActorLocation` self) (`self.TargetLocation`) _alpha)))))

(event `self.ReceiveTick`
  (params (DeltaSeconds :type "Float (single-precision)"))
  ;[1 1 1] Reverse target when finished and restart timer
  (if (== (`self.K2_GetActorLocation` self) (`self.TargetLocation`) :`ErrorTolerance` 1.0)
    (set `self.TempLocation` (`self.OriginalLocation`))
    (set `self.OriginalLocation` (`self.TargetLocation`))
    (set `self.TargetLocation` (`self.TempLocation`))
    (`self.Start Timer`)))

(fn `UserConstructionScript`)