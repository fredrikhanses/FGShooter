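; Laser wall obstacle that blinks on and off and damages the first-person character when it registers a hit.
; While the timer flag is set, Tick advances a frame-rate-dependent counter by a fixed step until it reaches the configured length.
; BlinkShield then flip-flops collision and visibility, plays a sound on one phase and restarts the timer.
; Deactivate hides the wall, disables its collision and stops the blinking.
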(event `Blink Timer`
  ;[1 1 1] Blink Timer
  (if (`self.StartBlinkTimer`)
    (if (< (`self.BlinkTimer`) (`self.BlinkTimerLength`))
      (set `self.BlinkTimer` (+ (`self.BlinkTimer`) 0.1))
      (else
        (set `self.StartBlinkTimer` false)
        (set `self.BlinkTimer` 0.0)
        (`self.Blink Shield`)))
    (else
      (set `self.BlinkTimer` 0.0))))

(event `Blink Shield`
  ;[1 1 1] Enable and disable shield
  (bind _isa (`/Engine/EditorBlueprintResources/StandardMacros.FlipFlop`)
    (:`A`
      _)
    (:`B`
      _))
  (`self.SetActorEnableCollision` _isa)
  (bind _returnvalue (not _isa))
  (`self.SetActorHiddenInGame` _returnvalue)
  (if _returnvalue
    (`GameplayStatics.PlaySoundAtLocation` "/Engine/VREditor/Sounds/UI/Dockable_Window_Close.Dockable_Window_Close" (`self.K2_GetActorLocation` self) (struct) 1.0 1.0 0.0 null null null))
  (set `self.StartBlinkTimer` true))

(event `self.ReceiveTick`
  (params (DeltaSeconds :type "Float (single-precision)"))
  ;[1 1 1] Start Timer
  (if (`self.StartBlinkTimer`)
    (`self.Blink Timer`)))

(event `self.StaticMeshComponent.OnComponentHit`
  (params (HitComponent :type "PrimitiveComponent Object Reference") (OtherActor :type "Actor Object Reference") (OtherComp :type "PrimitiveComponent Object Reference") (NormalImpulse :type "Vector Structure") (Hit :type "HitResult Structure (by ref)"))
  ;[1 1 1] Player hit
  (if (== (`GameplayStatics.GetObjectClass` OtherActor) "/Game/FGShooter/Player/FirstPersonCharacter.FirstPersonCharacter_C")
    (`GameplayStatics.ApplyDamage` OtherActor (`self.Damage`))))

(event `Deactivate`
  ;[1 1 1] Deactivate shield
  (`self.SetActorEnableCollision` false)
  (`self.SetActorHiddenInGame` true)
  (set `self.StartBlinkTimer` false))

(fn `UserConstructionScript`)