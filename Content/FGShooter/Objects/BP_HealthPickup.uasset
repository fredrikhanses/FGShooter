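; BP_HealthPickup is a pickup that restores health to the player on overlap.
; It reacts only to player character 0 and reads health from BP_GameState rather than from the character.
; When health is below the maximum, it adds HealthValue through AddHealth, plays the VR_teleport sound at the player's location and destroys itself.
; At full health the pickup stays in the world.
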(event `self.ReceiveActorBeginOverlap`
  (params (OtherActor :type "Actor Object Reference"))
  (if (== OtherActor (`GameplayStatics.GetPlayerCharacter` 0))
    (bind _asbp_game_state (cast `/Game/FGShooter/Core/BP_GameState` (`GameplayStatics.GetGameState`)))
    (if (< (`/Game/FGShooter/Core/BP_GameState.Health` _asbp_game_state) (`/Game/FGShooter/Core/BP_GameState.MaxHealth` _asbp_game_state))
      (`/Game/FGShooter/Core/BP_GameState.AddHealth` _asbp_game_state (`self.HealthValue`))
      (`GameplayStatics.PlaySoundAtLocation` "/Engine/VREditor/Sounds/VR_teleport.VR_teleport" (`self.K2_GetActorLocation` (`GameplayStatics.GetPlayerCharacter` 0)) (struct) 1.0 1.0 0.0 null null null)
      (`self.K2_DestroyActor`))))

(fn `UserConstructionScript`)