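; BP_LootableKey is a key pickup guarded by a breakable glass container and a switchable damaging shield.
; Projectile hits destroy the glass and enable physics on the key.
; Activate and Deactivate events toggle the shield's collision, visibility and sound, and the shield damages the player character on hit.
; StartInteract collects the key only when the glass is broken and the shield is off, hiding it and playing a sound.
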(event `self.GlassContainer.OnComponentHit`
  (params (HitComponent :type "PrimitiveComponent Object Reference") (OtherActor :type "Actor Object Reference") (OtherComp :type "PrimitiveComponent Object Reference") (NormalImpulse :type "Vector Structure") (Hit :type "HitResult Structure (by ref)"))
  ;[1 1 1] Break glass when shot
  (if (or (== (`GameplayStatics.GetObjectClass` OtherActor) "/Game/FGShooter/Player/FirstPersonProjectile.FirstPersonProjectile_C") (== (`GameplayStatics.GetObjectClass` OtherActor) "/Game/FGShooter/Player/FirstPersonSecondaryProjectile.FirstPersonSecondaryProjectile_C"))
    (set `self.GlassShot` true)
    (`ActorComponent.K2_DestroyComponent` (`self.GlassContainer`))
    (`PrimitiveComponent.SetSimulatePhysics` (`self.Key`) true)))

(event `/Game/FGShooter/Core/BPI_Interactable.Activate`
  (bind _shield (`self.Shield`))
  ;[1 1 1] Activate shield
  (set `self.Deactivated` false)
  (`PrimitiveComponent.SetCollisionEnabled` _shield "QueryOnly")
  (`SceneComponent.SetHiddenInGame` _shield false false)
  (bind _returnvalue (`GameplayStatics.SpawnSoundAtLocation` "/Game/StarterContent/Audio/Light02_Cue.Light02_Cue" (`self.K2_GetActorLocation` self) (struct) 3.0 1.0 0.0 null null))
  (set `self.AudioEffect` _returnvalue))

(event `self.Shield.OnComponentHit`
  (params (HitComponent :type "PrimitiveComponent Object Reference") (OtherActor :type "Actor Object Reference") (OtherComp :type "PrimitiveComponent Object Reference") (NormalImpulse :type "Vector Structure") (Hit :type "HitResult Structure (by ref)"))
  ;[1 1 1] Player takes damage when touching shield
  (if (== (`GameplayStatics.GetObjectClass` OtherActor) "/Game/FGShooter/Player/FirstPersonCharacter.FirstPersonCharacter_C")
    (`GameplayStatics.ApplyDamage` OtherActor (`self.Damage`))))

(event `/Game/FGShooter/Core/BPI_Interactable.Deactivate`
  (bind _shield (`self.Shield`))
  ;[1 1 1] Deactivate shield
  (set `self.Deactivated` true)
  (`PrimitiveComponent.SetCollisionEnabled` _shield "NoCollision")
  (`SceneComponent.SetHiddenInGame` _shield true false)
  (`AudioComponent.Stop` (`self.AudioEffect`)))

(event `/Game/FGShooter/Core/BPI_Interactable.StartInteract`
  (bind _key (`self.Key`))
  ;[1 1 1] Pick up key when able
  (if (`self.GlassShot`)
    (if (`self.Deactivated`)
      (set `self.KeyPickedUp` true)
      (`PrimitiveComponent.SetSimulatePhysics` _key false)
      (`PrimitiveComponent.SetCollisionEnabled` _key "NoCollision")
      (`SceneComponent.SetHiddenInGame` _key true false)
      (`GameplayStatics.PlaySoundAtLocation` "/Engine/EditorSounds/Notifications/CompileSuccess.CompileSuccess" (`self.K2_GetActorLocation` (`GameplayStatics.GetPlayerCharacter` 0)) (struct) 1.0 1.0 0.0 null null null))))

(fn `UserConstructionScript`)